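; Hatchet tool that chops harvestable large items and damages anything else it hits.
; Use plays first- and third-person chop montages; a notify sends the owner's arrow transform to a server sphere overlap.
; Non-lethal harvest hits award data-table resources by class name, scaled by tool type, tier, damage and randomness.
; Depleted items are swapped for their destruct class; harvest hits multicast particles and sound.
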(event Custom|GetRotationClient
  (bind (_location _rotation) (Class|BPISurvivalCharacter|GetArrowLocation(Message) (Components|GetOwner)))
  (CallFunction|ServerOverlap _location _rotation))

(event Custom|ServerOverlap
  (params (SpherePos :type Vector) (Rotation :type Rotator))
  (bind (_outactors _returnvalue) (Collision|SphereOverlapActors SpherePos 6e+01 (Utilities|Array|MakeArray "ObjectTypeQuery8" "ObjectTypeQuery3") 0 (Utilities|Array|MakeArray (Variables|Default|GetChar%20Ref))))
  (if _returnvalue
    (for _array_element _outactors
      (if (Utilities|DoesObjectImplementInterface _array_element "/Game/_Main/Blueprints/Interfaces/BPI_LargeItem.BPI_LargeItem_C")
        (CallFunction|HarvestFoliage 15.0 _array_element)
        (CallFunction|HitFXMulticast SpherePos Rotation)
        (else
          (Development|PrintString "HitPlayer")
          (Game|Damage|ApplyDamage _array_element 15.0 (Pawn|GetController (Variables|Default|GetChar%20Ref)) self "/Script/Engine.DamageType"))))
    (else
      (Development|PrintString "no hit"))))

(event Custom|HitFXMulticast
  (params (Location :type Vector) (Rotation :type Rotator))
  (bind _outhit (Collision|LineTraceByChannel Location (+ Location (* (Math|Vector|GetForwardVector Rotation) (Variables|Default|GetTraceDistance))) "TraceTypeQuery1" false 0 "None"))
  (Effects|SpawnEmitteratLocation "/Game/Realistic_Starter_VFX_Pack_Vol2/Particles/Hit/P_PickaxeHit.P_PickaxeHit" (.ImpactPoint (Collision|BreakHitResult _outhit)))
  (Audio|PlaySoundatLocation (Variables|Default|GetHitSound) Location "0, 0, 0" 1.0 1.0 0.0 "/Game/_Main/sounds/Harvesting/HarvestingAtt.HarvestingAtt" 0 0 0))

(event EventBeginPlay
  (|CallParentFunction) ; This node is disabled and will not be called.\nDrag off pins to build functionality.
)

(event Collision|EventActorBeginOverlap
  (params (OtherActor :type Actor%20Object%20Reference))
  (|CallParentFunction OtherActor) ; This node is disabled and will not be called.\nDrag off pins to build functionality.
)

(event EventTick
  (params (DeltaSeconds :type Float%20%28single-precision%29))
  (|CallParentFunction DeltaSeconds) ; This node is disabled and will not be called.\nDrag off pins to build functionality.
)

(event EventUseItemInterface
  (params (CharRef :type BP%20First%20Person%20Character%20Object%20Reference))
  (if (not (Variables|Default|GetIsSwinging?))
    (Variables|Default|SetIsSwinging? true)
    (bind _output_get (Variables|Default|SetChar%20Ref CharRef))
    (Class|BPISurvivalCharacter|FirstPersonMontage(Message) _output_get "/Game/Man/Animations/Hatchet_Chop_Montage.Hatchet_Chop_Montage")
    (Class|BPISurvivalCharacter|ThirdPersonMontage(Message) _output_get "/Game/Man/Animations/Hatchet_Chop_Montage.Hatchet_Chop_Montage")))

(event EventNotifyInterface
  (CallFunction|GetRotationClient))

(event EventEndAnimation
  (Variables|Default|SetIsSwinging? false))

(fn ConstructionScript
  (|CallParentFunction))

(fn HarvestFoliage
  (params (Damage :type Float%20%28double-precision%29) (Ref :type Actor%20Object%20Reference))
  (LocalVariables|SetLocalDamage Damage)
  (bind _ref (Class|BPILargeItem|GetLargeItemRef(Message) Ref))
  (Utilities|IsValid _ref
    (:Is%20Valid
      (bind _output_get (LocalVariables|SetLocalHealth (- (Variables|/Game/_Main/Blueprints/HarvestingSystem/BP_LargeItemMaster.BP_LargeItemMaster_C|GetHealth _ref) (LocalVariables|GetLocalDamage))))
      (Development|PrintString (Utilities|String|ToString(Float) _output_get))
      (if (<= (LocalVariables|GetLocalHealth) 0.0)
        (Development|PrintString "Tree is harvested")
        (bind _returnvalue (Utilities|GetDataTableRow "/Game/_Main/Blueprints/DataTables/DT_LargeItemResources.DT_LargeItemResources" (Utilities|String|StringToName (Utilities|GetClassDisplayName (Utilities|GetClass _ref))))
          (:then
            (LocalVariables|SetLocalDestructClass (.Class (Utilities|Struct|BreakS_LargeItem _returnvalue)))
            (LocalVariables|SetLocalTransform (Transformation|GetActorTransform _ref))
            (Actor|DestroyActor _ref)
            (Game|SpawnActorfromClass (LocalVariables|GetLocalDestructClass) (LocalVariables|GetLocalTransform) "Undefined" 0 (Transformation|GetActorForwardVector (Variables|Default|GetChar%20Ref)) 0)))
        (else
          (Variables|/Game/_Main/Blueprints/HarvestingSystem/BP_LargeItemMaster.BP_LargeItemMaster_C|SetHealth _ref (LocalVariables|GetLocalHealth))
          (bind _returnvalue_2 (Utilities|GetDataTableRow "/Game/_Main/Blueprints/DataTables/DT_LargeItemResources.DT_LargeItemResources" (Utilities|String|StringToName (Utilities|GetClassDisplayName (Utilities|GetClass _ref))))
            (:then
              (LocalVariables|SetGivenResources (.GivenItems (Utilities|Struct|BreakS_LargeItem _returnvalue_2)))
              (for _array_element (LocalVariables|GetGivenResources)
                (LocalVariables|SetLocalResourceQuantity (Math|Float|Truncate (|((((BaseVar*RateVar)*ToolTypeVar)*ToolTierVar)*DamageVar) (Math|Conversions|ToFloat(Integer) (.Quantity (Utilities|Struct|BreakS_ResourceStructure _array_element))) 1.0 (Math|Float|SelectFloat (Math|Random|RandomFloatinRange 0.2 0.4) (Math|Random|RandomFloatinRange 0.01 0.1) (Utilities|Enum|Equal(Enum) (.PrefferedToolType (Utilities|Struct|BreakS_ResourceStructure _array_element)) (Variables|Default|GetToolType))) (Utilities|Select :Index (Variables|Default|GetToolTier) :NewEnumerator0 (Math|Random|RandomFloatinRange 0.8 1.2) :NewEnumerator1 (Math|Random|RandomFloatinRange 1.2 1.6)) (LocalVariables|GetLocalDamage))))
                (if (not (<= (LocalVariables|GetLocalResourceQuantity) 0))
                  (bind _survivalcharref (Class|BPISurvivalCharacter|GetSurvivalCharRef(Message) (Variables|Default|GetChar%20Ref)))
                  (Default|HarvestItemonServer _survivalcharref (Utilities|Struct|MakeS_ResourceStructure (.ResourceID (Utilities|Struct|BreakS_ResourceStructure _array_element)) (LocalVariables|GetLocalResourceQuantity) "NewEnumerator0")))))))))))